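; Base enemy character Blueprint that handles health, hit reactions, a simple state value and death.
; Damage turns the enemy toward its causer, pushes it back via a timeline and plays a montage chosen by damage type.
; GetHitReaction also has side effects: it triggers the timeline-driven launch and switches airborne enemies to Swimming, or Falling for knockback.
; Landing handles knockback get-up and deferred state reset; death plays a montage and adjusts collision.
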(event `LaunchEnemy`
  (set `self.LauchLocation` (+ (`self.K2_GetActorLocation`) (0.0 0.0 250.0)))
  (bind (_direction _alpha) (`Timeline|Launch`)
    (:`Update`
      (`self.K2_SetActorLocation` (`KismetMathLibrary.VLerp` (`self.K2_GetActorLocation`) (`self.LauchLocation`) _alpha)))))

(event `Buffer`
  (params (Distance :type "Float (single-precision)"))
  (bind _returnvalue (`self.K2_GetActorLocation`))
  ;[0.05098 0.05098 0.05098] Buffer
  (`self.StopBuffer`)
  (if (!= Distance 0.0)
    (bind (_direction _alpha) (`Timeline|Timeline` :!via `PlayFromStart` :!label _label)
      (:`Update`
        (`self.K2_SetActorLocation` (`KismetMathLibrary.VLerp` _returnvalue (+ _returnvalue (* (* (`self.GetActorForwardVector`) -1.0) Distance)) _alpha) true)))))

(event `StopBuffer`
  ;[0.05098 0.05098 0.05098] Buffer
  (goto _label :!via `Stop`))

(event `self.ReceiveAnyDamage`
  (params (Damage :type "Float (single-precision)") (DamageType :type "DamageType Object Reference") (InstigatedBy :type "Controller Object Reference") (DamageCauser :type "Actor Object Reference"))
  (bind (_returnvalue_roll _returnvalue_pitch) (`KismetMathLibrary.BreakRotator` (`self.K2_GetActorRotation`)))
  (bind _charactermovement (`self.CharacterMovement`))
  (bind (_returnvalue_roll_2 _returnvalue_pitch_2 _returnvalue_yaw) (`KismetMathLibrary.BreakRotator` (`KismetMathLibrary.FindLookAtRotation` (`self.K2_GetActorLocation`) (`self.K2_GetActorLocation` DamageCauser))))
  (bind _output_get (set `self.Health` (- (`self.Health`) Damage)))
  (if (> _output_get 0.0)
    (bind _asbp_damage_type_main (cast `/Game/Bluepirnts/Character/DamageType/BP_DamageTypeMain` DamageType))
    (bind _damagetype (`/Game/Bluepirnts/Character/DamageType/BP_DamageTypeMain.DamageType` _asbp_damage_type_main))
    (bind _returnvalue (`self.GetHitReaction` _damagetype))
    (if (and (not (`self.IsCurrentStateEqualToAny` (`|MakeArray` "NewEnumerator3" :!type "/Game/Bluepirnts/Character/Enums/E_States Enum"))) (`KismetSystemLibrary.IsValid` _returnvalue))
      (`self.SetState` "NewEnumerator4")
      (`self.K2_SetActorRotation` (`KismetMathLibrary.MakeRotator` _returnvalue_roll _returnvalue_pitch _returnvalue_yaw))
      (if (and (not (`NavMovementComponent.IsFalling` _charactermovement)) (`CharacterMovementComponent.IsWalking` _charactermovement) (not (`NavMovementComponent.IsFlying` _charactermovement)) (not (`KismetArrayLibrary.Array_Contains` (`self.DamageTypeExempt`) _damagetype)))
        _
        (else
          _))
      (if (`KismetArrayLibrary.Array_Contains` (`self.DamageTypeExempt`) _damagetype)
        (`self.Buffer` 75.0)
        (else
          (`self.Buffer` 10.0)))
      (`self.PlayAnimMontage` _returnvalue))
    (else
      (`self.PerformDeath`))))

(event `ResetState`
  (bind _movementmode (`CharacterMovementComponent.MovementMode` (`self.CharacterMovement`)))
  (if (or (`|EnumEquality` _movementmode "MOVE_Falling") (`|EnumEquality` _movementmode "MOVE_Flying"))
    (set `self.bOnLandReset` true)
    (`CharacterMovementComponent.SetMovementMode` (`self.CharacterMovement`) "MOVE_Walking" 0)
    (else
      (`self.SetState` "NewEnumerator0"))))

(event `self.OnLanded`
  (params (Hit :type "HitResult Structure (by ref)"))
  (if (`self.bAirKnockback`)
    (set `self.bAirKnockback` false)
    (bind _notifyname (`|PlayMontage` (`self.Mesh`) (`self.HR_AirKnockback_OnLanded`))
      (:`then`
        (`CharacterMovementComponent.SetMovementMode` (`self.CharacterMovement`) "MOVE_Walking" 0))
      (:`OnNotifyBegin`
        (switch `name` _notifyname
          (:`GetUp`
            (`self.PlayAnimMontage` (`self.GetUpMontage`))))))
    (elif (`self.bOnLandReset`)
      (`CharacterMovementComponent.SetMovementMode` (`self.CharacterMovement`) "MOVE_Walking" 0)
      (set `self.bOnLandReset` false)
      (`self.ResetState`))))

(fn `GetHitReaction`
  (params (DamageType :type "/Game/Bluepirnts/Character/Enums/E_DamageTypes Enum" :default "NewEnumerator0"))
  (returns (ReturnValue :type "AnimMontage Object Reference"))
  (bind _charactermovement (`self.CharacterMovement`))
  (if (or (`NavMovementComponent.IsFlying` _charactermovement) (`NavMovementComponent.IsFalling` _charactermovement) (not (`CharacterMovementComponent.IsWalking` (`self.CharacterMovement`))))
    (`CharacterMovementComponent.SetMovementMode` (`self.CharacterMovement`) "MOVE_Swimming" 0)
    (switch `/Game/Bluepirnts/Character/Enums/E_DamageTypes` DamageType
      (:`NewEnumerator0`
        _)
      (:`NewEnumerator1`
        _)
      (:`NewEnumerator2`
        _)
      (:`NewEnumerator3`
        _)
      (:`NewEnumerator5`
        (`CharacterMovementComponent.SetMovementMode` (`self.CharacterMovement`) "MOVE_Falling" 0)
        (set `self.bAirKnockback` true)
        (return (`self.HR_AirKnockback`)))
      (:`NewEnumerator6`
        _))
    (return (`self.HR_Launch`))
    (else
      (switch `/Game/Bluepirnts/Character/Enums/E_DamageTypes` DamageType
        (:`NewEnumerator1`
          (return (`self.HR_R`)))
        (:`NewEnumerator2`
          (return (`self.HR_L`)))
        (:`NewEnumerator3`
          (return (`self.HR_Middle`)))
        (:`NewEnumerator4`
          (return (`self.HR_Knockdown`)))
        (:`NewEnumerator5`
          (return (`self.HR_Knockback`)))
        (:`NewEnumerator6`
          (`self.LaunchEnemy`)
          (return (`self.HR_Launch`)))))))

(fn `GetState`
  (returns (ReturnValue :type "/Game/Bluepirnts/Character/Enums/E_States Enum"))
  (return (`self.CurrentState`)))

(fn `IsCurrentStateEqualToAny`
  (params (StatesToCheck :type "Array of /Game/Bluepirnts/Character/Enums/E_States Enum (by ref)"))
  (returns (ReturnValue :type Boolean))
  (return (`KismetArrayLibrary.Array_Contains` StatesToCheck (`self.CurrentState`))))

(fn `PerformDeath`
  (bind _capsulecomponent (`self.CapsuleComponent`))
  (`self.SetState` "NewEnumerator3")
  (`self.PlayAnimMontage` (`self.DeathAnimMontage`))
  (`PrimitiveComponent.SetCollisionResponseToChannel` _capsulecomponent "ECC_Pawn" "ECR_Ignore")
  (`PrimitiveComponent.SetCollisionResponseToChannel` (`self.Mesh`) "ECC_Pawn" "ECR_Ignore")
  (`PrimitiveComponent.SetCollisionEnabled` (`self.Mesh`) "NoCollision")
  (`PrimitiveComponent.SetCollisionResponseToChannel` _capsulecomponent "ECC_WorldStatic" "ECR_Block")
  (`PrimitiveComponent.SetCollisionResponseToChannel` (`self.Mesh`) "ECC_WorldStatic" "ECR_Block")
  (`PrimitiveComponent.SetCollisionResponseToChannel` _capsulecomponent "ECC_WorldDynamic" "ECR_Block")
  (`PrimitiveComponent.SetCollisionEnabled` _capsulecomponent "PhysicsOnly"))

(fn `SetState`
  (params (NewState :type "/Game/Bluepirnts/Character/Enums/E_States Enum" :default "NewEnumerator0"))
  (if (`|EnumInequality` NewState (`self.CurrentState`))
    (set `self.CurrentState` NewState)))

(fn `UserConstructionScript`)